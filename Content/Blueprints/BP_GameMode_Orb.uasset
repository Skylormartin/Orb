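; Game mode that times runs through a level and records the best time for each level.
; StartTimer looks up the level index in BP_GameInstance from the map name minus its first two characters, then resets the clock.
; Tick accumulates world delta time while timing is active.
; StopTimer halts the clock and saves the time to the game instance if it is faster or the first recorded.
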(event `self.ReceiveTick`
  (params (DeltaSeconds :type "Float (single-precision)"))
  (if (`self.bIsTiming`)
    (set `self.CurrentTime` (+ (`self.CurrentTime`) (`GameplayStatics.GetWorldDeltaSeconds`)))))

(fn `CleanMapName`
  (returns (`Level Name` :type String))
  (bind _returnvalue (`GameplayStatics.GetCurrentLevelName` true))
  (return (`KismetStringLibrary.RightChop` _returnvalue 2)))

(fn `StartTimer`
  (bind _level_name (`self.CleanMapName`))
  (bind _asbp_game_instance (cast `/Game/Blueprints/BP_GameInstance` (`GameplayStatics.GetGameInstance`))
    (:`then`
      (set `self.LevelIndex` (`BlueprintMapLibrary.Map_Find` (`/Game/Blueprints/BP_GameInstance.LevelNameToIndex` _asbp_game_instance) _level_name))
      (set `self.CurrentTime` 0.0)
      (set `self.bIsTiming` true))
    (:`CastFailed`
      (`KismetSystemLibrary.PrintString` "CAST TO GAME INSTANCE FAILED" true true (struct :`R` 0.625 :`G` 0.033656 :`A` 1.0)))))

(fn `StopTimer`
  (set `self.bIsTiming` false)
  (bind _asbp_game_instance (cast `/Game/Blueprints/BP_GameInstance` (`GameplayStatics.GetGameInstance`)))
  (bind _besttimes (`/Game/Blueprints/BP_GameInstance.BestTimes` _asbp_game_instance))
  (bind (_value _returnvalue) (`BlueprintMapLibrary.Map_Find` _besttimes (`self.LevelIndex`)))
  (if (or (< (`self.CurrentTime`) _value) (not _returnvalue))
    (`BlueprintMapLibrary.Map_Add` _besttimes (`self.LevelIndex`) (`self.CurrentTime`))))

(fn `UserConstructionScript`)