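; Health component for target actors that tracks health and handles their death.
; ApplyDamage subtracts damage from CurrentHealth, clamped between zero and MaxHealth, and fires the OnDeath dispatcher at zero.
; The component binds its own handler to OnDeath on BeginPlay, which calls UpdateTargets on the cached BP_GameMode_Orb and destroys the owning actor.
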(event `self.ReceiveBeginPlay`
  (set `self.CurrentHealth` (`self.MaxHealth`))
  (set `self.isAlive` true)
  (add `self.OnDeath` (delegate `OnDeath_Event`))
  (bind _asbp_game_mode_orb (cast `/Game/Blueprints/BP_GameMode_Orb` (`GameplayStatics.GetGameMode`)))
  (set `self.As BP Game Mode Orb` _asbp_game_mode_orb))

(event `OnDeath_Event`
  (`/Game/Blueprints/BP_GameMode_Orb.UpdateTargets` (`self.As BP Game Mode Orb`))
  (`Actor.K2_DestroyActor` (`self.GetOwner`)))

(fn `ApplyDamage`
  (params (DamageAmount :type "Float (double-precision)"))
  (set `self.CurrentHealth` (`KismetMathLibrary.FClamp` (- (`self.CurrentHealth`) DamageAmount) 0.0 (`self.MaxHealth`)))
  (if (<= (`self.CurrentHealth`) 0.0)
    (set `self.isAlive` false)
    (`self.OnDeath`)))