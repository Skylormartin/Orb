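; BP_Orb is the player-controlled physics ball, rolled by camera-relative forces, with orbit camera, zoom and crosshair HUD.
; A capsule-trace ground check scales acceleration, gates horizontal speed clamping and surface-angled jumps, and switches on airborne spin impulses.
; Boost events add an impulse, temporarily raise max speed and animate FOV, while sprint input is disabled.
; ADS tightens the crosshair, a Granit component is added at BeginPlay, and Tick prints debug values.
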(event `EnhancedInput|/Game/Input/Orb/IA_Zoom`
  (params (ActionValue :type "Float (double-precision)") (ElapsedSeconds :type "Float (double-precision)") (TriggeredSeconds :type "Float (double-precision)") (InputAction :type "InputAction Object Reference" :default "/Game/Input/Orb/IA_Zoom.IA_Zoom"))
  (bind _springarm (`self.SpringArm`))
  ;[0 0 0] Camera Code
  ;;[0 0 0] Camera Zoom
  (:`Triggered`
    (set `SpringArmComponent.TargetArmLength` (`KismetMathLibrary.FClamp` (+ (* ActionValue (`self.Scroll to Zoom Magnitude`)) (`SpringArmComponent.TargetArmLength` _springarm)) 400.0 3000.0) _springarm)))

(event `self.ReceiveBeginPlay`
  ;[0 0.02604 0.000658] Begin Play
  (`|ExecutionSequence`
    (:`then_0`
      (bind _asplayer_controller (cast `PlayerController` (`self.GetController`)))
      (`EnhancedInputSubsystemInterface.AddMappingContext` (pcsubsystem `EnhancedInputLocalPlayerSubsystem` _asplayer_controller) "/Game/Input/Orb/IMC_Orb.IMC_Orb" 0 (struct)))
    (:`then_1`
      (set `self.Default FOV` (`CameraComponent.FieldOfView` (`self.Camera`))))
    (:`then_2`
      (bind _returnvalue (`|CreateWidget` "/Game/UI/WBP_Orb.WBP_Orb_C"))
      (bind _output_get (set `self.Orb HUD` _returnvalue))
      (`UserWidget.AddToViewport` _output_get 0))
    (:`then_3`
      (bind _returnvalue_2 (`AddComponent|NODE_AddBP_Granit_Component-0`))
      (set `self.Granit` _returnvalue_2))))

(event `EnhancedInput|/Game/Input/Orb/IA_Look`
  (params (ActionValue :type "Vector2D Structure") (ElapsedSeconds :type "Float (double-precision)") (TriggeredSeconds :type "Float (double-precision)") (InputAction :type "InputAction Object Reference" :default "/Game/Input/Orb/IA_Look.IA_Look"))
  (bind (_relativerotation_roll _relativerotation_pitch _relativerotation_yaw) (`KismetMathLibrary.BreakRotator` (`SceneComponent.RelativeRotation` (`self.SpringArm`))))
  (bind _returnvalue (+ ActionValue_X _relativerotation_yaw))
  (bind _returnvalue_2 (`KismetMathLibrary.FClamp` (+ ActionValue_Y _relativerotation_pitch) -89.0 75.0))
  ;[0 0 0] Camera Code
  ;;[0 0 0] Camera Rotation
  (:`Triggered`
    (`SceneComponent.K2_SetRelativeRotation` (`self.SpringArm`) (`KismetMathLibrary.MakeRotator` 0.0 _returnvalue_2 _returnvalue) false false)
    (`SceneComponent.K2_SetRelativeRotation` (`self.GranitSpringArm`) (`KismetMathLibrary.MakeRotator` 0.0 _returnvalue_2 _returnvalue) false false)))

(event `EnhancedInput|/Game/Input/Orb/IA_Roll`
  (params (ActionValue :type "Vector2D Structure") (ElapsedSeconds :type "Float (double-precision)") (TriggeredSeconds :type "Float (double-precision)") (InputAction :type "InputAction Object Reference" :default "/Game/Input/Orb/IA_Roll.IA_Roll"))
  (bind _camera (`self.Camera`))
  (bind (_returnvalue_x _returnvalue_y _returnvalue_z) (`KismetMathLibrary.BreakVector` (* (`self.Current Direction`) (`self.In Air Rot Speed`))))
  (bind _returnvalue (`KismetMathLibrary.Vector_Normal2D` (+ (* ActionValue_Y (`SceneComponent.GetForwardVector` _camera)) (* ActionValue_X (`SceneComponent.GetRightVector` _camera)))))
  ;[0 0 0] Movement Logic
  (:`Triggered`
    (set `self.Current Direction` _returnvalue)
    (`PrimitiveComponent.AddForce` (`self.Collision`) (* _returnvalue (`self.GetAccelerationForce`)) "None" false)
    (if (`self.Ground Check`)
      (`self.Debug Direction` (`self.Current Direction`))
      (`self.Clamp Velocity`)
      (else
        (`PrimitiveComponent.AddAngularImpulseInRadians` (`self.Collision`) (`KismetMathLibrary.MakeVector` (`self.Negate` _returnvalue_y) _returnvalue_x _returnvalue_z) "None" false) ; This little bit is so we can rotate efficiently when in the air
      ))))

(event `EnhancedInput|/Game/Input/Orb/IA_ADS`
  (params (ActionValue :type Boolean) (ElapsedSeconds :type "Float (double-precision)") (TriggeredSeconds :type "Float (double-precision)") (InputAction :type "InputAction Object Reference" :default "/Game/Input/Orb/IA_ADS.IA_ADS"))
  ;[0 0 0 0.5] ADS
  (:`Started`
    (set `self.isADS` true)
    (bind (_direction _alpha) (`Timeline|Timeline` :!label _label)
      (:`Update`
        (set `/Game/UI/WBP_Orb.CrosshairSpread` (`KismetMathLibrary.Lerp` 20.0 4.0 _alpha) (`self.Orb HUD`))
        (`CameraComponent.SetFieldOfView` (`self.Camera`) (`KismetMathLibrary.Lerp` (`self.Default FOV`) 75.0)))))
  (:`Completed`
    (set `self.isADS` false)
    (goto _label :!via `Reverse`)))

(event `EnhancedInput|/Game/Input/Orb/IA_Jump`
  (params (ActionValue :type Boolean) (ElapsedSeconds :type "Float (double-precision)") (TriggeredSeconds :type "Float (double-precision)") (InputAction :type "InputAction Object Reference" :default "/Game/Input/Orb/IA_Jump.IA_Jump"))
  (bind (_is_grounded_ _angled_jump_direction) (`self.Ground Check`))
  ;[0 0 0] Jump Logic
  (:`Triggered`
    (`/Engine/EditorBlueprintResources/StandardMacros.DoOnce` false :!label _label_2
      (:`Completed`
        (if _is_grounded_
          (`PrimitiveComponent.AddImpulse` (`self.Collision`) (* _angled_jump_direction (`self.Jump Force`)) "None" false)))))
  (:`Completed`
    (goto _label_2 :!via `Reset`)))

(event `/Game/Blueprints/BPI_Boost.Boost`
  (params (Direction :type "Vector Structure"))
  ;[0 0 0] Floor Boost Logic
  (bind _output_get (set `self.IsCurrentlyBoosting?` true))
  (if _output_get
    (set `self.Max Speed` 40000.0)
    (`PrimitiveComponent.AddImpulse` (`self.Collision`) (* Direction (`self.Boost Force`)) "None" false)
    (bind (_direction _boost_curve) (`Timeline|Boost FOV` :!via `PlayFromStart`)
      (:`Update`
        (`CameraComponent.SetFieldOfView` (`self.Camera`) (`KismetMathLibrary.Lerp` (`self.Default FOV`) (`self.BoostFOV`) _boost_curve)))
      (:`Finished`
        (set `self.IsCurrentlyBoosting?` false)
        (set `self.Max Speed` 26000.0)))))

(event `self.ReceiveTick`
  (params (DeltaSeconds :type "Float (single-precision)"))
  ;[0.002664 0.02083 0] DEBUG INFO: don't do anything else in event tick it's not performant
  (bind _returnvalue (`PrimitiveComponent.GetPhysicsLinearVelocity` (`self.Collision`) "None"))
  (`KismetSystemLibrary.PrintString` (`KismetStringLibrary.Concat_StrStr` "Current Velocity: " (`KismetStringLibrary.Conv_Vector2dToString` (`KismetMathLibrary.MakeVector2D` (.x _returnvalue) (.y _returnvalue)))) true false (struct :`G` 0.66 :`B` 1.0 :`A` 1.0) 0.0)
  (`KismetSystemLibrary.PrintString` (`KismetStringLibrary.Concat_StrStr` "Current Acceleration Force: " (`KismetStringLibrary.Conv_DoubleToString` (`self.GetAccelerationForce`))) true false (struct :`R` 1.0 :`G` 0.25235 :`A` 1.0) 0.0))

(event `EnhancedInput|/Game/Input/Orb/IA_Sprint`
  (params (ActionValue :type Boolean) (ElapsedSeconds :type "Float (double-precision)") (TriggeredSeconds :type "Float (double-precision)") (InputAction :type "InputAction Object Reference" :default "/Game/Input/Orb/IA_Sprint.IA_Sprint"))
  ;[0.05729 0 0] Boost Logic -- Disabled for now since it kinda conflicts with the floor boosts
)

(fn `Clamp Velocity`
  (bind (_returnvalue_x _returnvalue_y _returnvalue_z) (`KismetMathLibrary.BreakVector` (`self.GetVelocity`)))
  (bind _max_speed (`self.Max Speed`))
  (bind __ (`self.Negate` _max_speed))
  (`PrimitiveComponent.SetPhysicsLinearVelocity` (`self.Collision`) (`KismetMathLibrary.MakeVector` (`KismetMathLibrary.FClamp` _returnvalue_x __ _max_speed) (`KismetMathLibrary.FClamp` _returnvalue_y __ _max_speed) _returnvalue_z) false "None") ; - Clamp our orb velocity so we don't endlessly add speed\n- But we don't care about z velocity, so people can roll down fast
)

(fn `Debug Direction`
  (params (Direction :type "Vector Structure"))
  ;[0.7656 0 0] Debug direction visualization
  (if (`self.Debug Spheres`)
    (`KismetSystemLibrary.DrawDebugSphere` (+ (* Direction (200.0 200.0 0.0)) (`SceneComponent.K2_GetComponentLocation` (`self.Collision`))) 5.0 12 (struct :`G` 1.0 :`B` 0.043339 :`A` 1.0))))

(fn `GetAccelerationForce`
  (returns (Acceleration :type "Float (double-precision)"))
  (if (`self.Ground Check`)
    (if (or (`self.IsSprinting?`) (`self.IsCurrentlyBoosting?`))
      (return (* (`self.Acceleration Force`) 2.0))
      (else
        (return (`self.Acceleration Force`))))
    (else
      (return (/ (`self.Acceleration Force`) 2.0)))))

(fn `Ground Check`
  (returns (`Is Grounded?` :type Boolean) (`Angled Jump Direction` :type "Vector Structure"))
  (bind _returnvalue (`self.K2_GetActorLocation`))
  (bind _outhit (`KismetSystemLibrary.CapsuleTraceSingle` :`Start` _returnvalue :`End` (+ _returnvalue (`KismetMathLibrary.MakeVector` 0.0 0.0 (* (`SphereComponent.SphereRadius` (`self.Collision`)) -1.04))) :`Radius` 20.0 :`TraceChannel` "TraceTypeQuery1" :`DrawDebugType` "ForDuration" :`DrawTime` 0.01))
  (return (`GameplayStatics.BreakHitResult` _outhit) (`KismetMathLibrary.VLerp` (0.0 0.0 1.0) (`.Normal` (`GameplayStatics.BreakHitResult` _outhit)) 0.8)))

(fn `UserConstructionScript`)